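; BP_Martillo2 is a hammer pickup that the player carries to break a fragile box.
; Any actor overlap toggles an outline overlay, since the cast checks the player pawn rather than the overlapping actor.
; Interact registers it as the held item, disables physics and collision, and attaches it to the VR right controller or PC hand anchor.
; When PickupTrigger overlaps a BP_CajaFragil, both are destroyed and the held item is cleared.
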(event OnComponentBeginOverlap(PickupTrigger)
  (params (OverlappedComponent :type Primitive%20Component%20Object%20Reference) (OtherActor :type Actor%20Object%20Reference) (OtherComp :type Primitive%20Component%20Object%20Reference) (OtherBodyIndex :type Integer) (bFromSweep :type Boolean) (SweepResult :type Hit%20Result%20Structure%20%28by%20ref%29))
  (Utilities|Casting|CastToBP_CajaFragil OtherActor)
  (Actor|DestroyActor OtherActor)
  (Actor|DestroyActor)
  (bind _asbp_player_pawn (Utilities|Casting|CastToBP_PlayerPawn (Game|Player|GetPlayerPawn 0)))
  (Variables|/Game/Game/BP_PlayerPawn.BP_PlayerPawn_C|SetCurrentHeldItem%20 _asbp_player_pawn 0))

(event EventBeginPlay
  (|CallParentFunction) ; This node is disabled and will not be called.\nDrag off pins to build functionality.
)

(event Collision|EventActorBeginOverlap
  (params (OtherActor :type Actor%20Object%20Reference))
  (Utilities|Casting|CastToBP_PlayerPawn (Game|Player|GetPlayerPawn 0))
  (Rendering|Material|SetOverlayMaterial (Variables|Default|GetSM_Martillo) "/Game/Materials/Mi_Outline_mat_Inst.Mi_Outline_mat_Inst" :!class /Script/Engine.MeshComponent))

(event EventTick
  (params (DeltaSeconds :type Float%20%28single-precision%29))
  (|CallParentFunction DeltaSeconds) ; This node is disabled and will not be called.\nDrag off pins to build functionality.
)

(event Collision|EventActorEndOverlap
  (params (OtherActor :type Actor%20Object%20Reference))
  (Utilities|Casting|CastToBP_PlayerPawn (Game|Player|GetPlayerPawn 0))
  (Rendering|Material|SetOverlayMaterial (Variables|Default|GetSM_Martillo) 0 :!class /Script/Engine.MeshComponent))

(event EventInteract
  (bind _asbp_player_pawn (Utilities|Casting|CastToBP_PlayerPawn (Game|Player|GetPlayerPawn 0)))
  (if (== (Variables|/Game/Game/BP_PlayerPawn.BP_PlayerPawn_C|GetCurrentHeldItem%20 _asbp_player_pawn) 0)
    (Variables|/Game/Game/BP_PlayerPawn.BP_PlayerPawn_C|SetCurrentHeldItem%20 _asbp_player_pawn self)
    (if (Variables|Default|GetbIsPickedUp)
      (Development|PrintString "no")
      (else
        (Development|PrintString "si")
        (Variables|Default|SetbIsPickedUp true)
        (Physics|SetSimulatePhysics (Variables|Default|GetSM_Martillo) false)
        (Collision|SetCollisionEnabled (Variables|Default|GetSM_Martillo) "NoCollision")
        (bind _asbp_player_pawn_2 (Utilities|Casting|CastToBP_PlayerPawn (Game|Player|GetPlayerPawn 0)))
        (bind _output_get (Variables|Default|SetPlayerRef _asbp_player_pawn_2))
        (if (Variables|/Game/Game/BP_PlayerPawn.BP_PlayerPawn_C|GetIsVR _output_get)
          (Transformation|AttachComponentToComponent (Variables|/Game/Game/BP_PlayerPawn.BP_PlayerPawn_C|GetRightMotionController (Variables|Default|GetPlayerRef)) "None" "SnapToTarget" "SnapToTarget" "KeepWorld" true)
          (Transformation|SetActorRelativeRotation "0.000000,0.000000,90.000000")
          (Transformation|SetActorRelativeLocation "10.000000,0.000000,0.000000")
          (else
            (Transformation|AttachComponentToComponent (Variables|/Game/Game/BP_PlayerPawn.BP_PlayerPawn_C|GetPC_HandAnchor (Variables|Default|GetPlayerRef)) "None" "SnapToTarget" "SnapToTarget" "KeepWorld" true)
            (Transformation|SetActorRelativeRotation "-70.000000,0.000000,90.000000")))))))

(fn ConstructionScript
  (|CallParentFunction))

(fn SetHighlight)