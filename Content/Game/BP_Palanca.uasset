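; BP_Palanca is an interactable lever for non-VR players, meant to pitch with vertical mouse movement.
; Interact_1 sets IsGrabbed and records the mouse position; nothing here clears the grab.
; While grabbed, Tick adds the sensitivity-scaled Y delta to a clamped angle and applies it as relative pitch.
; Tick overwrites LastMouseY before computing that delta, so it evaluates to zero as wired.
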(event Custom|Interact_1
  (bind _returnvalue (Game|GetPlayerController 0))
  (bind (_locationx _locationy) (Game|Player|GetMousePosition _returnvalue))
  (bind _asbp_player_pawn (Utilities|Casting|CastToBP_PlayerPawn (Game|Player|GetPlayerPawn 0)))
  (if (not (Variables|/Game/Game/BP_PlayerPawn.BP_PlayerPawn_C|GetIsVR _asbp_player_pawn))
    (Variables|Default|SetbIsGrabbed%20 true)
    (Variables|Default|SetLastMouseX%20 _locationx)
    (Variables|Default|SetLastMouseY _locationy)))

(event EventBeginPlay
  (|CallParentFunction) ; This node is disabled and will not be called.\nDrag off pins to build functionality.
)

(event Collision|EventActorBeginOverlap
  (params (OtherActor :type Actor%20Object%20Reference)))

(event EventTick
  (params (DeltaSeconds :type Float%20%28single-precision%29))
  (bind _returnvalue (Game|GetPlayerController 0))
  (bind _returnvalue_2 (Transformation|GetActorRotation))
  (bind _locationy (Game|Player|GetMousePosition _returnvalue))
  (|CallParentFunction DeltaSeconds)
  (if (Variables|Default|GetbIsGrabbed%20)
    (Variables|Default|SetLastMouseY _locationy)
    (Variables|Default|SetCurrentAngle%20 (Math|Float|Clamp(Float) (+ (* (Variables|Default|GetSensibilidad) (- _locationy (Variables|Default|GetLastMouseY))) (Variables|Default|GetCurrentAngle%20)) (Variables|Default|GetMinAngle%20) (Variables|Default|GetMaxAngle%20)))
    (Transformation|SetActorRelativeRotation (Math|Rotator|MakeRotator (.roll _returnvalue_2) (Math|Float|Clamp(Float) (+ (* (Variables|Default|GetSensibilidad) (- _locationy (Variables|Default|GetLastMouseY))) (Variables|Default|GetCurrentAngle%20)) (Variables|Default|GetMinAngle%20) (Variables|Default|GetMaxAngle%20)) (.yaw _returnvalue_2)))))

(fn ConstructionScript
  (|CallParentFunction))