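; Game mode that tracks how many BP_Target actors remain and handles the win condition.
; On BeginPlay it counts all targets in the level into TargetsLeft.
; TargetEliminado decrements that count; at zero it switches the first BP_StartButton found into restart mode, re-arms it and plays a victory voice line.
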(event EventBeginPlay
  ;[1 1 1] Contar los Targets qie hay en el mapa
  (bind _outactors (Actor|GetAllActorsOfClass "/Game/Game/BP_Target.BP_Target_C"))
  (Variables|Default|SetTargetsLeft (Utilities|Array|Length _outactors)))

(fn ConstructionScript)

(fn TargetEliminado
  ;[1 1 1] Restamos a la cantidad total de enemigos y comprobamos si es 0 para cambiar el botón a modo resetear
  (Variables|Default|SetTargetsLeft (- (Variables|Default|GetTargetsLeft) 1))
  (if (<= (Variables|Default|GetTargetsLeft) 0)
    (bind _outactors (Actor|GetAllActorsOfClass "/Game/Game/BP_StartButton.BP_StartButton_C"))
    (Variables|/Game/Game/BP_StartButton.BP_StartButton_C|SetbReinicio (Utilities|Array|Get(acopy) _outactors) true)
    (Variables|/Game/Game/BP_StartButton.BP_StartButton_C|SetbUsed (Utilities|Array|Get(acopy) _outactors) false)
    (Default|RestartButtonChange (Utilities|Array|Get(acopy) _outactors))
    (Audio|PlaySound2D "/Game/Audio/S_VictoryVoice.S_VictoryVoice" 1.0 1.0 0.0 0 0)))