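; Shield pickup that attaches to the player's left hand when interacted with, supporting both VR and PC.
; Interact disables the mesh's physics and collision, attaches it to the left motion controller (with an offset) or PC hand anchor, then destroys the box collision.
; Overlap events toggle an outline overlay material until pickup, checking the player pawn's class rather than the overlapping actor.
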(event Collision|EventActorBeginOverlap
  (params (OtherActor :type Actor%20Object%20Reference))
  ;[1 1 1] Resaltar Objeto
  (Utilities|Casting|CastToBP_PlayerPawn (Game|Player|GetPlayerPawn 0))
  (if (not (Variables|Default|GetIsPickedUp))
    (Rendering|Material|SetOverlayMaterial (Variables|Default|GetSM_Shield) "/Game/Materials/Mi_Outline_mat_Inst.Mi_Outline_mat_Inst" :!class /Script/Engine.MeshComponent)))

(event Collision|EventActorEndOverlap
  (params (OtherActor :type Actor%20Object%20Reference))
  ;[1 1 1] Resaltar Objeto
  (Utilities|Casting|CastToBP_PlayerPawn (Game|Player|GetPlayerPawn 0))
  (Rendering|Material|SetOverlayMaterial (Variables|Default|GetSM_Shield) 0 :!class /Script/Engine.MeshComponent))

(event EventInteract
  ;[1 1 1] Coger objetos dependiendo si es PC o VR
  (if (not (Variables|Default|GetIsPickedUp))
    (Variables|Default|SetIsPickedUp true)
    (Physics|SetSimulatePhysics (Variables|Default|GetSM_Shield) false)
    (Collision|SetCollisionEnabled (Variables|Default|GetSM_Shield) "NoCollision")
    (bind _asbp_player_pawn (Utilities|Casting|CastToBP_PlayerPawn (Game|Player|GetPlayerPawn 0)))
    (bind _output_get (Variables|Default|SetPlayerRef _asbp_player_pawn))
    (if (Variables|/Game/Game/BP_PlayerPawn.BP_PlayerPawn_C|GetIsVR _output_get)
      (Transformation|AttachComponentToComponent (Variables|/Game/Game/BP_PlayerPawn.BP_PlayerPawn_C|GetLeftMotionController (Variables|Default|GetPlayerRef)) "None" "SnapToTarget" "SnapToTarget" "KeepWorld" true)
      (Transformation|SetActorRelativeLocation "20.000000,0.000000,0.000000")
      (Components|DestroyComponent (Variables|Default|GetBoxCollision))
      (else
        (Transformation|AttachComponentToComponent (Variables|/Game/Game/BP_PlayerPawn.BP_PlayerPawn_C|GetPC_HandAnchorLeft (Variables|Default|GetPlayerRef)) "None" "SnapToTarget" "SnapToTarget" "KeepWorld" true)
        (Components|DestroyComponent (Variables|Default|GetBoxCollision))))))

(fn ConstructionScript
  (|CallParentFunction))