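; BP_Gun is a pickup gun that shoots targets in both VR and PC play.
; Interact disables its physics and attaches it to the player's right motion controller or PC hand anchor, while overlaps toggle an outline.
; Shot, limited by a short cooldown, spawns a short-lived bullet alongside a muzzle line trace.
; The trace places a brief impact decal, destroys any BP_Target hit and notifies BP_GameMode.
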(event Custom|Shot
  (bind _muzzle_ (Variables|Default|GetMuzzle%20))
  (bind _muzzle__2 (Variables|Default|GetMuzzle%20))
  (bind _returnvalue (Transformation|GetWorldLocation _muzzle_))
  (bind _returnvalue_2 (Math|Vector|GetForwardVector _muzzle__2))
  (if (Variables|Default|GetbIsPickedUp%20)
    (if (Variables|Default|GetbCanShoot%20)
      (Variables|Default|SetbCanShoot%20 false)
      (Audio|PlaySound2D "/Game/Audio/S_laser_sound.S_laser_sound" 1.0 1.0 0.0 0 0 false)
      (bind _returnvalue_3 (Game|SpawnActorfromClass "/Game/Game/BP_BaseBullet.BP_BaseBullet_C" (Math|Transform|MakeTransform _returnvalue (Math|Conversions|RotationFromXVector _returnvalue_2) "1.000000,1.000000,1.000000") "Undefined" "MultiplyWithRoot" 0 0))
      (Actor|SetLifeSpan _returnvalue_3 2.0)
      (bind (_outhit _returnvalue_4) (Collision|LineTraceByChannel _returnvalue (+ _returnvalue (* _returnvalue_2 (Math|Conversions|ToVector(Float) 2e+03))) "TraceTypeQuery1" false 0 "None"))
      (Utilities|FlowControl|Sequence
        (:then_0
          (Utilities|FlowControl|Delay 0.2)
          (Variables|Default|SetbCanShoot%20 true))
        (:then_1
          (if _returnvalue_4
            (bind _returnvalue_5 (Rendering|Decal|SpawnDecalatLocation "/Game/Materials/M_T_TCom_Broke_Mat.M_T_TCom_Broke_Mat" "8.000000,8.000000,8.000000" (.Location (Collision|BreakHitResult _outhit)) (Math|Rotator|MakeRotfromX (.ImpactNormal (Collision|BreakHitResult _outhit))) 0.0))
            (Utilities|FlowControl|Sequence
              (:then_0
                (Utilities|FlowControl|Delay 0.2)
                (Components|DestroyComponent _returnvalue_5))
              (:then_1
                (bind _asbp_target (Utilities|Casting|CastToBP_Target (.HitActor (Collision|BreakHitResult _outhit))))
                (Audio|PlaySoundatLocation "/Game/Audio/S_crate-break.S_crate-break" (Transformation|GetActorLocation _asbp_target) "0, 0, 0" 1.0 1.0 0.0 0 0 0 0)
                (Actor|DestroyActor _asbp_target)
                (bind _asbp_game_mode (Utilities|Casting|CastToBP_GameMode (Game|GetGameMode)))
                (Default|TargetEliminado _asbp_game_mode)))))))))

(event Collision|EventActorBeginOverlap
  (params (OtherActor :type Actor%20Object%20Reference))
  (Utilities|Casting|CastToBP_PlayerPawn (Game|Player|GetPlayerPawn 0))
  (Rendering|Material|SetOverlayMaterial (Variables|Default|GetCube) "/Game/Materials/Mi_Outline_mat_Inst.Mi_Outline_mat_Inst" :!class /Script/Engine.MeshComponent))

(event Collision|EventActorEndOverlap
  (params (OtherActor :type Actor%20Object%20Reference))
  (Utilities|Casting|CastToBP_PlayerPawn (Game|Player|GetPlayerPawn 0))
  (Rendering|Material|SetOverlayMaterial (Variables|Default|GetCube) 0 :!class /Script/Engine.MeshComponent))

(event EventInteract
  (bind _asbp_player_pawn (Utilities|Casting|CastToBP_PlayerPawn (Game|Player|GetPlayerPawn 0)))
  (if (== (Variables|/Game/Game/BP_PlayerPawn.BP_PlayerPawn_C|GetCurrentHeldItem%20 _asbp_player_pawn) 0)
    (Variables|/Game/Game/BP_PlayerPawn.BP_PlayerPawn_C|SetCurrentHeldItem%20 _asbp_player_pawn self)
    (if (Variables|Default|GetbIsPickedUp%20)
      (Development|PrintString "no")
      (else
        (Development|PrintString "si")
        (Variables|Default|SetbIsPickedUp%20 true)
        (Physics|SetSimulatePhysics (Variables|Default|GetSM_Gun) false)
        (Collision|SetCollisionEnabled (Variables|Default|GetSM_Gun) "NoCollision")
        (bind _asbp_player_pawn_2 (Utilities|Casting|CastToBP_PlayerPawn (Game|Player|GetPlayerPawn 0)))
        (bind _output_get (Variables|Default|SetPlayerRef%20 _asbp_player_pawn_2))
        (if (Variables|/Game/Game/BP_PlayerPawn.BP_PlayerPawn_C|GetIsVR _output_get)
          (Transformation|AttachComponentToComponent (Variables|/Game/Game/BP_PlayerPawn.BP_PlayerPawn_C|GetRightMotionController (Variables|Default|GetPlayerRef%20)) "None" "SnapToTarget" "SnapToTarget" "KeepWorld" true)
          (Transformation|SetActorRelativeLocation "20.000000,0.000000,0.000000")
          (else
            (Transformation|AttachComponentToComponent (Variables|/Game/Game/BP_PlayerPawn.BP_PlayerPawn_C|GetPC_HandAnchor (Variables|Default|GetPlayerRef%20)) "None" "SnapToTarget" "SnapToTarget" "KeepWorld" true)))))))

(fn ConstructionScript
  (|CallParentFunction))