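; Player pawn supporting VR and desktop play, choosing movement, look and interaction behavior by headset detection at BeginPlay.
; On desktop it moves camera-relative at fixed height; interaction line-traces from the camera, or right controller in VR, to call BP_Interactable.
; Holding teleport redraws a predicted spline-mesh arc from the left controller each Tick; release moves to the navmesh-projected point, offset by camera position.
; Shooting forwards to a held BP_Gun.
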(event Input|EnhancedActionEvents|EnhancedInputActionIA_Shot
  (params (ActionValue :type Boolean) (ElapsedSeconds :type Float%20%28double-precision%29) (TriggeredSeconds :type Float%20%28double-precision%29) (InputAction :type Input%20Action%20Object%20Reference :default "/Game/Game/Input/IA_Shot.IA_Shot"))
  (bind _currenthelditem_ (Variables|Default|GetCurrentHeldItem%20))
  (if (== _currenthelditem_ "/Game/Game/BP_Gun.BP_Gun")
    _
    (else
      _))
  (bind _asbp_gun (Utilities|Casting|CastToBP_Gun _currenthelditem_))
  (Default|Shot _asbp_gun))

(event Input|EnhancedActionEvents|EnhancedInputActionIA_Interact
  (params (ActionValue :type Boolean) (ElapsedSeconds :type Float%20%28double-precision%29) (TriggeredSeconds :type Float%20%28double-precision%29) (InputAction :type Input%20Action%20Object%20Reference :default "/Game/Game/Input/IA_Interact.IA_Interact"))
  (if (Variables|Default|GetIsVR)
    (CallFunction|InteractVR)
    (else
      (CallFunction|InteractPC))))

(event Input|EnhancedActionEvents|EnhancedInputActionIA_Look
  (params (ActionValue :type Vector%202D%20Structure) (ElapsedSeconds :type Float%20%28double-precision%29) (TriggeredSeconds :type Float%20%28double-precision%29) (InputAction :type Input%20Action%20Object%20Reference :default "/Game/Game/Input/IA_Look.IA_Look"))
  (bind _sensibilidad (Variables|Default|GetSensibilidad))
  (bind _returnvalue (* ActionValue _sensibilidad))
  (if (not (Variables|Default|GetIsVR))
    (Transformation|AddRelativeRotation (Variables|Default|GetMainCamera) (Math|Rotator|MakeRotator 0.0 (.y _returnvalue) (.x _returnvalue)) false false)))

(event Input|EnhancedActionEvents|EnhancedInputActionIA_Move
  (params (ActionValue :type Vector :default "0, 0, 0") (ElapsedSeconds :type Float%20%28double-precision%29) (TriggeredSeconds :type Float%20%28double-precision%29) (InputAction :type Input%20Action%20Object%20Reference :default "/Game/Game/Input/IA_Move.IA_Move"))
  (if (not (Variables|Default|GetIsVR))
    (CallFunction|MovePC (.x ActionValue) (.y ActionValue))))

(event Input|EnhancedActionEvents|EnhancedInputActionIA_Teleport
  (params (ActionValue :type Boolean) (ElapsedSeconds :type Float%20%28double-precision%29) (TriggeredSeconds :type Float%20%28double-precision%29) (InputAction :type Input%20Action%20Object%20Reference :default "/Game/Game/Input/IA_Teleport.IA_Teleport"))
  (:Started
    (Variables|Default|SetbIsAimingTeleport%20 true))
  (:Completed
    (Variables|Default|SetbIsAimingTeleport%20 false)))

(event EventBeginPlay
  (bind _returnvalue (Class|HeadMountedDisplayFunctionLibrary|IsHeadMountedDisplayEnabled))
  (Utilities|FlowControl|Sequence
    (:then_0
      (bind _asplayer_controller (Utilities|Casting|CastToPlayerController (Pawn|GetController)))
      (Input|AddMappingContext (PlayerController|LocalPlayerSubsystems|GetEnhancedInputLocalPlayerSubsystem _asplayer_controller) "/Game/Game/Input/IMC_Game.IMC_Game" 0 "(bIgnoreAllPressedKeysUntilRelease=True,bForceImmediately=False,bNotifyUserSettings=False)"))
    (:then_1
      (Variables|Default|SetIsVR _returnvalue)
      (if _returnvalue
        (Class|HeadMountedDisplayFunctionLibrary|SetTrackingOrigin "LocalFloor")))))

(event EventTick
  (params (DeltaSeconds :type Float%20%28single-precision%29))
  (bind _leftmotioncontroller (Variables|Default|GetLeftMotionController))
  (Utilities|FlowControl|Sequence
    (:then_0
      (if (Variables|Default|GetbIsAimingTeleport%20)
        (CallFunction|TeleportArc (Transformation|GetWorldLocation _leftmotioncontroller) (Math|Vector|GetForwardVector _leftmotioncontroller))
        (goto _label Reset)
        (else
          (Utilities|FlowControl|DoOnce true :!label _label
            (:Completed
              (Transformation|SetActorLocation (Variables|Default|GetTeleportLocation%20) false false)
              (CallFunction|ClearArc))))))))

(fn ConstructionScript)

(fn MovePC
  (params (B :type Float%20%28double-precision%29) (B2 :type Float%20%28double-precision%29))
  (bind _returnvalue (Transformation|GetActorLocation))
  (bind _maincamera (Variables|Default|GetMainCamera))
  (bind _returnvalue_2 (Math|Vector|GetForwardVector _maincamera))
  (bind _returnvalue_3 (Math|Vector|GetRightVector _maincamera))
  (bind _returnvalue_4 (* _returnvalue_3 B2))
  (bind _returnvalue_5 (* _returnvalue_2 B))
  (bind _returnvalue_6 (Utilities|MultiplyLocationPerSpeed _returnvalue_5))
  (bind _returnvalue_7 (Utilities|MultiplyLocationPerSpeed _returnvalue_4))
  (bind _returnvalue_8 (+ _returnvalue _returnvalue_6 _returnvalue_7 ""))
  (Transformation|SetActorLocation (Math|Vector|MakeVector (.x _returnvalue_8) (.y _returnvalue_8) 1.6e+02) false false))

(fn TeleportArc
  (params (StartingLocation :type Vector) (FowardVector :type Vector))
  (bind _splinemesh (Variables|Default|GetSplineMesh))
  (bind _maincamera (Variables|Default|GetMainCamera))
  (bind _relativelocation (Variables|/Script/Engine.SceneComponent|GetRelativeLocation _maincamera))
  (bind (_outhit _outpathpositions _outlasttracedestination _returnvalue) (Class|GameplayStatics|BlueprintPredictProjectilePathbyTraceChannel StartingLocation (* FowardVector 500) true 0.0 "ECC_WorldStatic" false 0 "None"))
  (LocalVariables|SetPaths _outpathpositions)
  (for _array_element _splinemesh
    (Components|DestroyComponent _array_element))
  (Utilities|Array|Clear _splinemesh)
  (for _index (range 1 (- (Utilities|Array|Length (LocalVariables|GetPaths)) 1))
    (bind _returnvalue_2 (AddComponent|AddSplineMeshComponent true))
    (Utilities|Array|Add (Variables|Default|GetSplineMesh) _returnvalue_2)
    (SplineMesh|SetStartandEnd _returnvalue_2 (Utilities|Array|Get(acopy) (LocalVariables|GetPaths) (- _index 1)) "0, 0, 0" (Utilities|Array|Get(acopy) (LocalVariables|GetPaths) _index) "0, 0, 0" true :!class /Script/Engine.SplineMeshComponent))
  (if _returnvalue
    (if (.ReturnValue (AI|Navigation|ProjectPointtoNavigation _outlasttracedestination 0 0 "0, 0, 0"))
      (Variables|Default|SetTeleportLocation%20 (Math|Vector|MakeVector (- (.x (.ProjectedLocation (AI|Navigation|ProjectPointtoNavigation _outlasttracedestination 0 0 "0, 0, 0"))) (.x _relativelocation)) (- (.y (.ProjectedLocation (AI|Navigation|ProjectPointtoNavigation _outlasttracedestination 0 0 "0, 0, 0"))) (.y _relativelocation)) (.z (.ProjectedLocation (AI|Navigation|ProjectPointtoNavigation _outlasttracedestination 0 0 "0, 0, 0")))))
      (else
        (Variables|Default|SetTeleportLocation%20 (Transformation|GetActorLocation))))
    (else
      (Variables|Default|SetTeleportLocation%20 (Transformation|GetActorLocation)))))

(fn ClearArc
  (bind _splinemesh (Variables|Default|GetSplineMesh))
  (for _array_element _splinemesh
    (Components|DestroyComponent _array_element))
  (Utilities|Array|Clear _splinemesh))

(fn InteractPC
  (bind _maincamera (Variables|Default|GetMainCamera))
  (bind _returnvalue (Transformation|GetWorldLocation _maincamera))
  (bind (_outhit _returnvalue_2) (Collision|LineTraceByChannel _returnvalue (+ _returnvalue (* (Math|Vector|GetForwardVector (Variables|Default|GetMainCamera)) 250)) "TraceTypeQuery1" false 0 "None"))
  (if _returnvalue_2
    (bind _asbp_interactable (Utilities|Casting|CastToBP_Interactable (.HitActor (Collision|BreakHitResult _outhit))))
    (Default|Interact _asbp_interactable)))

(fn InteractVR
  (bind _rightmotioncontroller (Variables|Default|GetRightMotionController))
  (bind _returnvalue (Transformation|GetWorldLocation _rightmotioncontroller))
  (bind (_outhit _returnvalue_2) (Collision|LineTraceByChannel _returnvalue (+ _returnvalue (* (Math|Vector|GetForwardVector _rightmotioncontroller) 250)) "TraceTypeQuery1" false 0 "None"))
  (if _returnvalue_2
    (bind _asbp_interactable (Utilities|Casting|CastToBP_Interactable (.HitActor (Collision|BreakHitResult _outhit))))
    (Default|Interact _asbp_interactable)))