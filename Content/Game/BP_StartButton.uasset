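; BP_StartButton is an interactable button that unblocks and opens a door, or reloads LS_TestRoom when its Reinicio flag is set.
; On first use it destroys the blocking door, plays a sound and runs a timeline that lowers the button mesh, calling OpenDoor on every update.
; RestartButtonChange applies the restart material and resets the mesh position, but does not set Reinicio itself.
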(event EventInteract
  (bind _doorref (Variables|Default|GetDoorRef))
  (if (Variables|Default|GetbReinicio)
    (Game|OpenLevel(byObjectReference) "/Game/Game/Levels/LS_TestRoom.LS_TestRoom")
    (elif (not (Variables|Default|GetbUsed))
      (Variables|Default|SetbUsed true)
      (Actor|DestroyActor (Variables|Default|GetBlockDoorRef))
      (Audio|PlaySoundatLocation "/Game/Audio/S_DoorOpen.S_DoorOpen" "0, 0, 0" "0, 0, 0" 1.0 1.0 0.0 0 0 0 0)
      (bind _alpha (Timeline|TL_BajarBoton Play)
        (:Update
          (Transformation|SetRelativeLocation (Variables|Default|GetSM_Button) (Math|Vector|Lerp(Vector) "0, 0, 0" "0.000000,0.000000,-15.000000" _alpha) false false)
          (if (!= _doorref 0)
            (Default|OpenDoor _doorref)))))))

(fn ConstructionScript
  (|CallParentFunction))

(fn RestartButtonChange
  (bind _sm_button (Variables|Default|GetSM_Button))
  (Rendering|Material|SetMaterial _sm_button 0 "/Game/Materials/M_RestartButton.M_RestartButton")
  (Transformation|SetRelativeLocation _sm_button "0, 0, 0" false false))